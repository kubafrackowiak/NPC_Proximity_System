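; BP_AwarenessSensor is an awareness sensor that shows on a text label whether something is inside its detection volume.
; Begin overlap on DetectionVolume sets StatusLabel to the alert text and color, and end overlap switches it to the end text and color.
; It is purely event-driven, with no filtering of the overlapping actor and no count of overlaps, so any exit clears the alert.
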(event `self.DetectionVolume.OnComponentBeginOverlap`
  (params (OverlappedComponent :type "PrimitiveComponent Object Reference") (OtherActor :type "Actor Object Reference") (OtherComp :type "PrimitiveComponent Object Reference") (OtherBodyIndex :type Integer) (bFromSweep :type Boolean) (SweepResult :type "HitResult Structure (by ref)"))
  (`TextRenderComponent.K2_SetText` (`self.StatusLabel`) (`self.AlertText`))
  (`TextRenderComponent.SetTextRenderColor` (`self.StatusLabel`) (`self.AlertColor`)))

(event `self.DetectionVolume.OnComponentEndOverlap`
  (params (OverlappedComponent :type "PrimitiveComponent Object Reference") (OtherActor :type "Actor Object Reference") (OtherComp :type "PrimitiveComponent Object Reference") (OtherBodyIndex :type Integer))
  (`TextRenderComponent.K2_SetText` (`self.StatusLabel`) (`self.EndText`))
  (`TextRenderComponent.SetTextRenderColor` (`self.StatusLabel`) (`self.EndColor`)))

(fn `UserConstructionScript`)